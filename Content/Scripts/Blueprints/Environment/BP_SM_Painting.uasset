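; BP_SM_Painting is an environment painting actor that sets the static mesh of its SwapPainting component on BeginPlay.
; The DefineType flag selects between a fixed mesh from TypePool at the SpecificType index and a random pick from that pool.
; The random pick uses a hardcoded range of five entries rather than the pool's length.
; The construction script is empty, so the swap happens only at runtime.
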(event `self.ReceiveBeginPlay`
  (if (`self.DefineType`)
    (`self.SetSpecificType`)
    (else
      (`self.RandomizeType`))))

(fn `RandomizeType`
  (`StaticMeshComponent.SetStaticMesh` (`self.SwapPainting`) (`|GetArrayItem` (`self.TypePool`) (`KismetMathLibrary.RandomInteger` 5))))

(fn `SetSpecificType`
  (`StaticMeshComponent.SetStaticMesh` (`self.SwapPainting`) (`|GetArrayItem` (`self.TypePool`) (`self.SpecificType`))))

(fn `UserConstructionScript`)