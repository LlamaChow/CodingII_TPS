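; Wall environment Blueprint that sets the mesh of its ReplaceableWall component when play begins.
; If DefineWall is set, it uses the WallType mesh at the SpecificWall index; otherwise it picks one at random.
; DoubleSided walls draw randomly from only the first two WallType entries, while other walls draw from the first four.
; The construction script is empty, so the chosen mesh is applied only at runtime.
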(event `self.ReceiveBeginPlay`
  (if (`self.DefineWall`)
    (`self.SetSpecificWall`)
    (else
      (`self.RandomizeWallType`))))

(fn `RandomizeWallType`
  (if (`self.DoubleSided`)
    (`StaticMeshComponent.SetStaticMesh` (`self.ReplaceableWall`) (`|GetArrayItem` (`self.WallType`) (`KismetMathLibrary.RandomInteger` 2)))
    (else
      (`StaticMeshComponent.SetStaticMesh` (`self.ReplaceableWall`) (`|GetArrayItem` (`self.WallType`) (`KismetMathLibrary.RandomInteger` 4))))))

(fn `SetSpecificWall`
  (`StaticMeshComponent.SetStaticMesh` (`self.ReplaceableWall`) (`|GetArrayItem` (`self.WallType`) (`self.SpecificWall`))))

(fn `UserConstructionScript`)