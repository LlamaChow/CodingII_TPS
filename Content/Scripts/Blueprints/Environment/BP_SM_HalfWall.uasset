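; BP_SM_HalfWall is an environment half-wall Blueprint that sets the mesh of its ReplacableWall component when play begins.
; If DefineType is set, it uses the WallTypes entry at SpecificType; otherwise it picks randomly from the first three entries.
; The construction script is empty, so the mesh swap happens only at runtime.
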(event `self.ReceiveBeginPlay`
  (if (`self.DefineType`)
    (`self.SetSpecific`)
    (else
      (`self.RandomizeType`))))

(fn `RandomizeType`
  (`StaticMeshComponent.SetStaticMesh` (`self.ReplacableWall`) (`|GetArrayItem` (`self.WallTypes`) (`KismetMathLibrary.RandomInteger` 3))))

(fn `SetSpecific`
  (`StaticMeshComponent.SetStaticMesh` (`self.ReplacableWall`) (`|GetArrayItem` (`self.WallTypes`) (`self.SpecificType`))))

(fn `UserConstructionScript`)