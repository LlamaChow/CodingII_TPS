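; Environment beam actor that chooses its mesh variant when play begins.
; By default it swaps the replaceable beam to a random mesh from the first five BeamTypes entries, or to SpecificType when DefineType is set.
; The Horizontal flag forces the defined path, which hides and disables collision on the replaceable beam and reveals a separate horizontal beam with collision enabled.
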(event `self.ReceiveBeginPlay`
  (if (`self.Horizontal`)
    (set `self.SpecificType` 5)
    (set `self.DefineType` true))
  (if (`self.DefineType`)
    (`self.SetSpecific`)
    (else
      (`self.RandomizeType`))))

(fn `RandomizeType`
  (`StaticMeshComponent.SetStaticMesh` (`self.ReplacableBeam`) (`|GetArrayItem` (`self.BeamTypes`) (`KismetMathLibrary.RandomInteger` 5))))

(fn `SetSpecific`
  (bind _replacablebeam (`self.ReplacableBeam`))
  (bind _horizontalbeam (`self.HorizontalBeam`))
  (if (`self.Horizontal`)
    (`SceneComponent.SetVisibility` _replacablebeam false false)
    (`PrimitiveComponent.SetCollisionEnabled` _replacablebeam "NoCollision")
    (`SceneComponent.SetHiddenInGame` _horizontalbeam false false)
    (`PrimitiveComponent.SetCollisionEnabled` _horizontalbeam "QueryAndPhysics")
    (else
      (`StaticMeshComponent.SetStaticMesh` (`self.ReplacableBeam`) (`|GetArrayItem` (`self.BeamTypes`) (`self.SpecificType`))))))

(fn `UserConstructionScript`)